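; BP_GameActor is a game actor with basic health, damage and death handling.
; BeginPlay sets HP to MaxHP, and GetDamage subtracts incoming damage, calling Death once HP drops strictly below zero, so exactly zero HP survives.
; Death simply destroys the actor, and the Other argument of GetDamage is unused.
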(event EventBeginPlay
  (Variables|Default|SetHP (Variables|Default|GetMaxHP)))

(event Collision|EventActorBeginOverlap
  (params (OtherActor :type Actor%20Object%20Reference)))

(event EventTick
  (params (DeltaSeconds :type Float%20%28single-precision%29)))

(fn ConstructionScript)

(fn GetDamage
  (params (damage :type Float%20%28single-precision%29) (other :type Actor%20Object%20Reference))
  (bind _output_get (Variables|Default|SetHP (- (Variables|Default|GetHP) damage)))
  (if (< _output_get 0.0)
    (CallFunction|Death)))

(fn Death
  (Actor|DestroyActor))