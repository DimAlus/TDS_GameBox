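; BP_MapBase is a grid map actor that lays out a floor of cells and marks a spawn cell.
; The construction script adds a flattened static mesh per cell over Size, scaled to WidthCell and lowered by HeightToEath.
; The cell at StartPos gets a different material from the rest.
; GetStartPos converts that cell to a world position by offsetting the actor location, ignoring rotation and the height drop.
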(event EventBeginPlay)

(event Collision|EventActorBeginOverlap
  (params (OtherActor :type Actor%20Object%20Reference)))

(event EventTick
  (params (DeltaSeconds :type Float%20%28single-precision%29)))

(fn ConstructionScript
  (bind _size (Variables|Default|Getsize))
  (bind _widthcell (Variables|Default|GetwidthCell))
  (bind _startpos (Variables|Default|GetstartPos))
  (bind _returnvalue (* _widthcell 0.009))
  (for _index (range 0 (.y _size)) ; row
    (for _index_2 (range 0 (.x _size)) ; column
      (bind _returnvalue_2 (AddComponent|AddStaticMeshComponent false (Math|Transform|MakeTransform (Math|Vector|MakeVector (* _index_2 _widthcell) (* _index _widthcell) (* (Variables|Default|GetheightToEath) -1.0)) "0, 0, 0" (Math|Vector|MakeVector _returnvalue _returnvalue 0.05))))
      (if (and (== _index (.y _startpos)) (== _index_2 (.x _startpos))) ; if is spawn position
        (Rendering|Material|SetMaterial _returnvalue_2 0 "/Engine/EngineMaterials/EditorBrushMaterial.EditorBrushMaterial")
        (else
          (Rendering|Material|SetMaterial _returnvalue_2 0 "/Engine/VREditor/UI/DiscMaterial.DiscMaterial"))))))

(fn GetStartPos
  (return (+ (Transformation|GetActorLocation) (* (Math|Conversions|ToVector(Float) (Variables|Default|GetstartPos)) (Variables|Default|GetwidthCell)))))