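; Pistol-shotgun weapon Blueprint that fires several bolts per shot.
; Its Shoting override calls the parent, then spawns a configurable number of bolts at the Parent actor's location and attaches them to God.OwnerTemp.
; Each bolt is initialized with the aim, enemy class, damage, lifetime and an angle error for spread.
; Shot and the construction script only defer to the parent class, and the default events are disabled.
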(event EventBeginPlay
  (|CallParentFunction) ; This node is disabled and will not be called.\nDrag off pins to build functionality.
)

(event Collision|EventActorBeginOverlap
  (params (OtherActor :type Actor%20Object%20Reference))
  (|CallParentFunction OtherActor) ; This node is disabled and will not be called.\nDrag off pins to build functionality.
)

(event EventTick
  (params (DeltaSeconds :type Float%20%28single-precision%29))
  (|CallParentFunction DeltaSeconds) ; This node is disabled and will not be called.\nDrag off pins to build functionality.
)

(fn ConstructionScript
  (|CallParentFunction))

(fn Shot
  (params (Aim :type Vector :default "0, 0, 0"))
  (|CallParentFunction Aim))

(fn Shoting
  (params (Aim :type Vector :default "0, 0, 0"))
  (|CallParentFunction Aim)
  (for _index (range 1 (Variables|Default|GetcountBolts))
    (bind _returnvalue (Game|SpawnActorfromClass (Variables|Default|GetboltClass) (Math|Conversions|ToTransform(Vector) (Transformation|GetActorLocation (Variables|Default|Getparent))) "AlwaysSpawn" 0 0))
    (Transformation|AttachActorToActor _returnvalue (Variables|/Game/Blueprints/BP_PlayerPawn.BP_PlayerPawn_C|GetownerTemp (Variables|Default|GetGod)) "None" "KeepRelative" "KeepRelative" "KeepRelative" true)
    (Default|InitBolt _returnvalue (Variables|Default|GetGod) (Variables|Default|GetenemyClass) (Variables|Default|Getdamage) Aim (Variables|Default|GetlifeBolts) (Variables|Default|GetangleError) (Variables|Default|Getparent))))