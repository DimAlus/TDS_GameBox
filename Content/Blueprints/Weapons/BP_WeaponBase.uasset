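; Base weapon Blueprint that provides cooldown-gated shooting and owner setup for weapons.
; InitWeapon initializes the weapon and stores its Parent, then passes whether that owner derives from BP_PlayerBase to an empty SettingEnemyClass hook.
; Shot calls Shoting when CanShot allows it; Shoting here only restarts the cooldown, which Tick counts down.
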(event EventBeginPlay
  (|CallParentFunction))

(event Collision|EventActorBeginOverlap
  (params (OtherActor :type Actor%20Object%20Reference))
  (|CallParentFunction OtherActor))

(event EventTick
  (params (DeltaSeconds :type Float%20%28single-precision%29))
  (|CallParentFunction DeltaSeconds)
  ;[1 1 1] Smalling cooldown
  (if (> (Variables|Default|GetactiveCooldown) 0.0)
    (Variables|Default|SetactiveCooldown (- (Variables|Default|GetactiveCooldown) DeltaSeconds))))

(fn ConstructionScript)

(fn Shot
  (params (Aim :type Vector))
  (if (Utilities|CanShot)
    (CallFunction|Shoting Aim)))

(fn SetParent
  (params (parent :type BP%20Game%20Actor%20Object%20Reference))
  (bind _output_get (Variables|Default|Setparent parent))
  (CallFunction|SettingEnemyClass (Utilities|ClassIsChildOf (Utilities|GetClass _output_get) "/Game/Blueprints/Player/BP_PlayerBase.BP_PlayerBase_C")))

(fn Shoting
  (params (Aim :type Vector))
  (Variables|Default|SetactiveCooldown (Variables|Default|Getcooldown)))

(fn SettingEnemyClass
  (params (isPlayer :type Boolean)))

(fn InitWeapon
  (params (God :type BP%20Player%20Pawn%20Object%20Reference) (Parent :type BP%20Game%20Actor%20Object%20Reference))
  (CallFunction|Init God)
  (CallFunction|SetParent Parent))

(fn IsCanShot
  (return (Utilities|CanShot)))