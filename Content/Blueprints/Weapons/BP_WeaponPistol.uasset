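; Pistol weapon, a child Blueprint that fires bolt projectiles for either the player or an enemy.
; Shoting runs the parent logic, then spawns BoltClass at the Parent actor's location, passes it EnemyClass and calls its Shot with aim and damage.
; SettingEnemyClass picks the bolt's target class from IsPlayer: BP_Enemy for the player, BP_PlayerBase otherwise.
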(event EventBeginPlay
  (|CallParentFunction) ; This node is disabled and will not be called.\nDrag off pins to build functionality.
)

(event Collision|EventActorBeginOverlap
  (params (OtherActor :type Actor%20Object%20Reference))
  (|CallParentFunction OtherActor) ; This node is disabled and will not be called.\nDrag off pins to build functionality.
)

(event EventTick
  (params (DeltaSeconds :type Float%20%28single-precision%29))
  (|CallParentFunction DeltaSeconds) ; This node is disabled and will not be called.\nDrag off pins to build functionality.
)

(fn ConstructionScript
  (|CallParentFunction))

(fn Shoting
  (params (Aim :type Vector :default "0, 0, 0"))
  (|CallParentFunction Aim)
  (bind _returnvalue (Game|SpawnActorfromClass (Variables|Default|GetboltClass) (Math|Conversions|ToTransform(Vector) (Transformation|GetActorLocation (Variables|Default|Getparent))) "AlwaysSpawn" 0 0))
  (Variables|/Game/Blueprints/Weapons/BP_BoltBase.BP_BoltBase_C|SetenemyClass _returnvalue (Variables|Default|GetenemyClass))
  (Default|Shot _returnvalue Aim (Variables|Default|Getdamage)))

(fn SettingEnemyClass
  (params (isPlayer :type Boolean))
  (if isPlayer
    (Variables|Default|SetenemyClass "/Game/Blueprints/Enemyes/BP_Enemy.BP_Enemy_C")
    (else
      (Variables|Default|SetenemyClass "/Game/Blueprints/Player/BP_PlayerBase.BP_PlayerBase_C"))))