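; Base Blueprint for weapon bolts that detect overlaps with enemies, leaving the shot and hit behavior to be overridden.
; InitBolt runs Init with God, stores the enemy class, damage, life, error and parent, then calls Shot with the aim.
; On overlap, actors matching the enemy class are cast to BP_GameActor and passed to HitEnemy.
; Shot and HitEnemy are empty here.
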(event EventBeginPlay
  (|CallParentFunction))

(event EventTick
  (params (DeltaSeconds :type Float%20%28single-precision%29))
  (|CallParentFunction DeltaSeconds))

(event Collision|EventActorBeginOverlap
  (params (OtherActor :type Actor%20Object%20Reference))
  (|CallParentFunction OtherActor)
  (if (Utilities|ClassIsChildOf (Utilities|GetClass OtherActor) (Variables|Default|GetenemyClass))
    (bind _asbp_game_actor (Utilities|Casting|CastToBP_GameActor OtherActor))
    (CallFunction|HitEnemy _asbp_game_actor)))

(fn ConstructionScript)

(fn Shot
  (params (Aim :type Vector)))

(fn HitEnemy
  (params (enemy :type BP%20Game%20Actor%20Object%20Reference)))

(fn InitBolt
  (params (God :type BP%20Player%20Pawn%20Object%20Reference) (enemyClass :type BP%20Game%20Actor%20Class%20Reference) (damage :type Float%20%28single-precision%29) (Aim :type Vector) (life :type Float%20%28single-precision%29) (error :type Float%20%28single-precision%29) (parent :type BP%20Game%20Actor%20Object%20Reference))
  (CallFunction|Init God)
  (Variables|Default|SetenemyClass enemyClass)
  (Variables|Default|Setdamage damage)
  (Variables|Default|Setlife life)
  (Variables|Default|Seterror error)
  (Variables|Default|Setparent parent)
  (CallFunction|Shot Aim))