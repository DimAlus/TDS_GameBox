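; Bolt projectile for weapons, built on a parent bullet class, that flies straight and damages the enemies it hits.
; Shot normalizes the aim vector and rotates it about Z by a random spread from AngleError to set the travel direction.
; Tick moves the actor along that direction with a swept offset and destroys it when its Life countdown runs out.
; HitEnemy passes a mass-scaled impulse and damage to the enemy.
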(event EventBeginPlay)

(event EventTick
  (params (DeltaSeconds :type Float%20%28single-precision%29))
  (CallFunction|Move DeltaSeconds)
  (bind _output_get (Variables|Default|Setlife (- (Variables|Default|Getlife) DeltaSeconds)))
  (if (< _output_get 0.0)
    (Actor|DestroyActor)))

(fn ConstructionScript
  (|CallParentFunction))

(fn Shot
  (params (Aim :type Vector :default "0, 0, 0"))
  (|CallParentFunction Aim)
  (Variables|Default|Setdir (Math|Vector|RotateVectorAroundAxis (Math|Vector|Normalize Aim) (|(((rand*2)-1)*angle) (Math|Random|RandomFloat) (Variables|Default|GetangleError)) "0,0.000000,1.000000")))

(fn HitEnemy
  (params (enemy :type BP%20Game%20Actor%20Object%20Reference))
  (bind _self self)
  (|CallParentFunction enemy)
  (Default|Touch enemy _self (* (Variables|Default|Getdir) (Variables|Default|Getmass)))
  (Default|GetDamage enemy (Variables|Default|Getdamage) _self))

(fn Move
  (params (deltaTime :type Float%20%28single-precision%29))
  (Transformation|AddActorWorldOffset (* (Variables|Default|Getdir) (* deltaTime (Variables|Default|Getspeed))) true))