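; BP_BoltSword is a melee-style bolt weapon that sweeps around its yaw axis and damages enemies it hits.
; InitBolt extends the parent setup, stores the normalized aim direction and orients the actor along it.
; Tick rotates the actor with sweep at Speed and counts down Angle, calling Death when it drops below zero.
; HitEnemy pushes the enemy along the aim direction scaled by Mass and applies Damage.
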(event EventBeginPlay
  (|CallParentFunction) ; This node is disabled and will not be called.\nDrag off pins to build functionality.
)

(event Collision|EventActorBeginOverlap
  (params (OtherActor :type Actor%20Object%20Reference))
  (|CallParentFunction OtherActor) ; This node is disabled and will not be called.\nDrag off pins to build functionality.
)

(event EventTick
  (params (DeltaSeconds :type Float%20%28single-precision%29))
  (bind _speed (Variables|Default|Getspeed))
  (bind _returnvalue (* DeltaSeconds _speed))
  (|CallParentFunction DeltaSeconds)
  (Transformation|AddActorLocalRotation (Math|Rotator|MakeRotator 0.0 0.0 _returnvalue) true false)
  (bind _output_get (Variables|Default|Setangle (- (Variables|Default|Getangle) _returnvalue)))
  (if (< _output_get 0.0)
    (CallFunction|Death)))

(fn ConstructionScript
  (|CallParentFunction))

(fn InitBolt
  (params (God :type BP%20Player%20Pawn%20Object%20Reference) (enemyClass :type BP%20Game%20Actor%20Class%20Reference) (damage :type Float%20%28single-precision%29) (Aim :type Vector :default "0, 0, 0") (life :type Float%20%28single-precision%29) (error :type Float%20%28single-precision%29) (parent :type BP%20Game%20Actor%20Object%20Reference))
  (|CallParentFunction God enemyClass damage Aim life error parent)
  (Variables|Default|Setdir (Math|Vector|Normalize Aim))
  (Transformation|SetActorRelativeRotation (Math|Conversions|RotationFromXVector Aim) false true))

(fn HitEnemy
  (params (enemy :type BP%20Game%20Actor%20Object%20Reference))
  (bind _self self)
  (|CallParentFunction enemy)
  (Default|Touch enemy _self (* (Variables|Default|Getdir) (Variables|Default|Getmass)))
  (Default|GetDamage enemy (Variables|Default|Getdamage) _self))