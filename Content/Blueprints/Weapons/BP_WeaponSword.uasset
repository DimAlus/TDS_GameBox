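; BP_WeaponSword is a sword weapon that overrides Shoting and SettingEnemyClass to deliver its attack.
; Shoting calls the parent, spawns a BoltClass actor attached to the weapon at zero relative offset, then initializes it with damage, aim, life and targeting data.
; SettingEnemyClass makes the target class BP_EnemyBase for player wielders and BP_PlayerBase otherwise.
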(event EventBeginPlay
  (|CallParentFunction) ; This node is disabled and will not be called.\nDrag off pins to build functionality.
)

(event Collision|EventActorBeginOverlap
  (params (OtherActor :type Actor%20Object%20Reference))
  (|CallParentFunction OtherActor) ; This node is disabled and will not be called.\nDrag off pins to build functionality.
)

(event EventTick
  (params (DeltaSeconds :type Float%20%28single-precision%29))
  (|CallParentFunction DeltaSeconds) ; This node is disabled and will not be called.\nDrag off pins to build functionality.
)

(fn ConstructionScript
  (|CallParentFunction))

(fn Shoting
  (params (Aim :type Vector :default "0, 0, 0"))
  (|CallParentFunction Aim)
  (bind _returnvalue (Game|SpawnActorfromClass (Variables|Default|GetboltClass) (Math|Transform|MakeTransform "0, 0, 0") "AlwaysSpawn" 0 0))
  (Transformation|AttachActorToActor _returnvalue self "None" "KeepRelative" "KeepRelative" "KeepRelative" true)
  (Default|InitBolt _returnvalue (Variables|Default|GetGod) (Variables|Default|GetenemyClass) (Variables|Default|Getdamage) Aim (Variables|Default|Getlife) 0.0 (Variables|Default|Getparent)))

(fn SettingEnemyClass
  (params (isPlayer :type Boolean))
  (if isPlayer
    (Variables|Default|SetenemyClass "/Game/Blueprints/Enemyes/BP_EnemyBase.BP_EnemyBase_C")
    (else
      (Variables|Default|SetenemyClass "/Game/Blueprints/Player/BP_PlayerBase.BP_PlayerBase_C"))))