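; BP_BoltSwordBig is a bolt weapon Blueprint, apparently a large sword variant, that overrides its parent class's InitBolt and Move.
; InitBolt runs the inherited setup, then rotates the actor to face the aim vector.
; Move offsets the Parent actor, rather than the bolt itself, along Dir by Speed and delta time without sweeping, provided Parent is valid.
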(event EventBeginPlay
  (|CallParentFunction) ; This node is disabled and will not be called.\nDrag off pins to build functionality.
)

(event Collision|EventActorBeginOverlap
  (params (OtherActor :type Actor%20Object%20Reference))
  (|CallParentFunction OtherActor) ; This node is disabled and will not be called.\nDrag off pins to build functionality.
)

(event EventTick
  (params (DeltaSeconds :type Float%20%28single-precision%29))
  (|CallParentFunction DeltaSeconds) ; This node is disabled and will not be called.\nDrag off pins to build functionality.
)

(fn ConstructionScript
  (|CallParentFunction))

(fn Move
  (params (deltaTime :type Float%20%28single-precision%29))
  (bind _parent (Variables|Default|Getparent))
  (Utilities|IsValid _parent
    (:Is%20Valid
      (Transformation|AddActorWorldOffset _parent (* (Variables|Default|Getdir) (* deltaTime (Variables|Default|Getspeed)))))))

(fn InitBolt
  (params (God :type BP%20Player%20Pawn%20Object%20Reference) (enemyClass :type BP%20Game%20Actor%20Class%20Reference) (damage :type Float%20%28single-precision%29) (Aim :type Vector :default "0, 0, 0") (life :type Float%20%28single-precision%29) (error :type Float%20%28single-precision%29) (parent :type BP%20Game%20Actor%20Object%20Reference))
  (|CallParentFunction God enemyClass damage Aim life error parent)
  (Transformation|SetActorRotation (Math|Conversions|RotationFromXVector Aim) true))