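; Base enemy actor that spawns attached weapons, fires them at players and steers itself to its preferred combat range.
; On a timer it picks the player nearest the weapons' average ideal distance and aims for a point at that range, randomly rotated around the target.
; Each tick, every ready weapon independently targets a player within its own range.
; Movement integrates velocity with acceleration, slowing and touch impulses, without sweeping.
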(event EventBeginPlay
  (bind _god (Variables|Default|GetGod))
  (|CallParentFunction)
  (Variables|Default|Setttf (Variables|Default|GetticksToThink))
  (Utilities|IsValid _god
    (:Is%20Valid
      (CallFunction|Init _god))))

(event EventTick
  (params (DeltaSeconds :type Float%20%28single-precision%29))
  (|CallParentFunction DeltaSeconds)
  (CallFunction|TicktoThink DeltaSeconds)
  (CallFunction|Shot)
  (CallFunction|ChangeVelocity)
  (Transformation|AddActorWorldOffset (* (Variables|Default|Getvelocity) DeltaSeconds)))

(fn ConstructionScript
  (|CallParentFunction))

(fn Think
  (bind _target (CallFunction|GetIdealPlayer (Transformation|GetActorLocation) -1.0 -1.0 (Variables|Default|GetbestLengthToEnemy)))
  (bind _output_get (Variables|Default|SetTarget _target))
  (Utilities|IsValid _output_get
    (:Is%20Valid
      (Variables|Default|SetAimToMove (+ (Transformation|GetActorLocation _output_get) (* (Math|Vector|RotateVectorAroundAxis (Math|Vector|Normalize (- (Transformation|GetActorLocation) (Transformation|GetActorLocation _output_get))) (Math|Random|RandomFloatinRange -2e+01 2e+01) "0, 0,1.000000") (Variables|Default|GetbestLengthToEnemy)))))))

(fn SpawnWeapons
  (bind _weapons (Variables|Default|Getweapons))
  (for _array_element (Variables|Default|GetweaponsClasses)
    (if (Utilities|IsValidClass _array_element)
      (bind _returnvalue (Game|SpawnActorfromClass _array_element (Math|Transform|MakeTransform "0, 0, 0") "AlwaysSpawn" 0 0))
      (Transformation|AttachActorToActor _returnvalue self "None" "KeepRelative" "KeepRelative" "KeepRelative" true)
      (Utilities|Array|Add _weapons _returnvalue)
      (Default|InitWeapon _returnvalue (Variables|Default|GetGod) self)
      (else
        (Utilities|Array|Add _weapons 0)))))

(fn Shot
  (for _array_element (Variables|Default|Getweapons)
    (if (Utilities|IsValid _array_element)
      (bind _canshot (Default|IsCanShot _array_element))
      (if _canshot
        (CallFunction|Shoting _array_element)))))

(fn Shoting
  (params (weapon :type BP%20Weapon%20Base%20Object%20Reference))
  (bind _target (CallFunction|ThinkWeaponTarget weapon))
  (Utilities|IsValid _target
    (:Is%20Valid
      (Default|Shot weapon (- (Transformation|GetActorLocation _target) (Transformation|GetActorLocation weapon))))))

(fn ThinkWeaponTarget
  (params (weapon :type BP%20Weapon%20Base%20Object%20Reference))
  (bind _target (CallFunction|GetIdealPlayer (Transformation|GetActorLocation) (Variables|/Game/Blueprints/Weapons/BP_WeaponBase.BP_WeaponBase_C|GetdistanceMin weapon) (Variables|/Game/Blueprints/Weapons/BP_WeaponBase.BP_WeaponBase_C|GetdistanceMax weapon) (Variables|/Game/Blueprints/Weapons/BP_WeaponBase.BP_WeaponBase_C|GetdistanceIdeal weapon)))
  (return _target))

(fn TicktoThink
  (params (DeltaTime :type Float%20%28single-precision%29))
  (bind _output_get (Variables|Default|Setttf (- (Variables|Default|Getttf) DeltaTime)))
  (if (< _output_get 0.0)
    (Variables|Default|Setttf (Variables|Default|GetticksToThink))
    (CallFunction|Think)))

(fn Init
  (params (God :type BP%20Player%20Pawn%20Object%20Reference))
  (|CallParentFunction God)
  (CallFunction|SpawnWeapons)
  (bind _length (CallFunction|BestLength))
  (Variables|Default|SetbestLengthToEnemy _length))

(fn Death
  (for _array_element (Variables|Default|Getweapons)
    (Utilities|IsValid _array_element
      (:Is%20Valid
        (CallFunction|Death _array_element))))
  (|CallParentFunction))

(fn BestLength
  (for _array_element (Variables|Default|Getweapons)
    (Utilities|IsValid _array_element
      (:Is%20Valid
        (LocalVariables|Setlen (+ (Variables|/Game/Blueprints/Weapons/BP_WeaponBase.BP_WeaponBase_C|GetdistanceIdeal _array_element) (LocalVariables|Getlen)))
        (Math|Integer|IncrementInt (LocalVariables|Getcount)))))
  (if (> (LocalVariables|Getcount) 0)
    (return (/ (LocalVariables|Getlen) (Math|Conversions|ToFloat(Integer) (LocalVariables|Getcount))))
    (else
      (return 0.0))))

(fn GetIdealPlayer
  (params (pos :type Vector) (minDistance :type Float%20%28single-precision%29) (maxDistance :type Float%20%28single-precision%29) (idealDistance :type Float%20%28single-precision%29))
  (bind _players (Default|GetPlayers (Variables|Default|GetGod)))
  (for (_array_element _array_index) _players
    (if (|(((min<0)||(max<0))||((len>=min)&&(len<=max))) (Utilities|Lengthto pos _array_element) minDistance maxDistance)
      (if (== (LocalVariables|GetminIndex) -1)
        (LocalVariables|SetminLength (|(abs((a-b))) (Utilities|Lengthto pos _array_element) idealDistance) :!label _label)
        (LocalVariables|SetminIndex _array_index)
        (elif (< (|(abs((a-b))) (Utilities|Lengthto pos _array_element) idealDistance) (LocalVariables|GetminLength))
          (goto _label)))))
  (if (== (LocalVariables|GetminIndex) -1)
    (return 0)
    (else
      (return (Utilities|Array|Get(acopy) _players (LocalVariables|GetminIndex))))))

(fn ChangeVelocity
  (bind _output_get (LocalVariables|Settemp (+ (Variables|Default|Getvelocity) (Utilities|VectortoLength (- (Variables|Default|GetAimToMove) (Transformation|GetActorLocation)) (Variables|Default|GetspeedUp)))))
  (Variables|Default|Setvelocity (- (LocalVariables|Gettemp) (Utilities|VectortoLength (LocalVariables|Gettemp) (Math|Float|Min(Float) (Math|Vector|VectorLength _output_get) (Variables|Default|Getslowing))))))

(fn Touch
  (params (other :type BP%20Game%20Actor%20Object%20Reference) (impulse :type Vector :default "0, 0, 0"))
  (|CallParentFunction other impulse)
  (Variables|Default|Setvelocity (+ (* impulse 5e+01) (Variables|Default|Getvelocity))))