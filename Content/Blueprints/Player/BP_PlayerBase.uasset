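; Base class for player characters that either act as the controlled player or as AI companions following God's active player.
; Movement is a 2D velocity with boost, speed cap, slowdown and touch impulses, applied each tick as a swept offset.
; Companions periodically re-aim at a randomised point around the main player and auto-fire each ready weapon at the enemy closest to its ideal range.
; Init spawns and attaches weapons; Death notifies God and kills them.
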(event EventBeginPlay
  (|CallParentFunction))

(event Collision|EventActorBeginOverlap
  (params (OtherActor :type Actor%20Object%20Reference))
  (|CallParentFunction OtherActor))

(event EventTick
  (params (DeltaSeconds :type Float%20%28single-precision%29))
  (|CallParentFunction DeltaSeconds)
  (CallFunction|TicktoThink DeltaSeconds)
  (if (Variables|Default|GetisPlayer)
    _
    (else
      (CallFunction|TryShoting)))
  (CallFunction|ChangeVelocity)
  (Transformation|AddActorWorldOffset (Math|Conversions|ToVector(Vector2D) (Variables|Default|Getvelocity)) true))

(fn ConstructionScript)

(fn ChangeVelocity
  (bind _maxvelocity (Variables|Default|GetmaxVelocity))
  (if (Variables|Default|GetisPlayer)
    _
    (elif (> (Math|Vector|VectorLength (+ (Math|Conversions|ToVector(Vector2D) (Variables|Default|Getvelocity)) (Utilities|VectortoLength (- (Variables|Default|GetAimToMove) (Transformation|GetActorLocation)) (Variables|Default|Getboost)))) _maxvelocity)
      (Variables|Default|Setvelocity (Math|Conversions|ToVector2D(Vector) (Utilities|VectortoLength (+ (Math|Conversions|ToVector(Vector2D) (Variables|Default|Getvelocity)) (Utilities|VectortoLength (- (Variables|Default|GetAimToMove) (Transformation|GetActorLocation)) (Variables|Default|Getboost))) _maxvelocity)))
      (else
        (Variables|Default|Setvelocity (Math|Conversions|ToVector2D(Vector) (+ (Math|Conversions|ToVector(Vector2D) (Variables|Default|Getvelocity)) (Utilities|VectortoLength (- (Variables|Default|GetAimToMove) (Transformation|GetActorLocation)) (Variables|Default|Getboost))))))))
  (CallFunction|Slowdown))

(fn AddVelocity
  (params (vel :type Vector%202D%20Structure))
  (bind _maxvelocity (Variables|Default|GetmaxVelocity))
  (if (> (Math|Vector2D|Vector2DLength (+ (Variables|Default|Getvelocity) (* vel (Variables|Default|Getboost)))) _maxvelocity)
    (Variables|Default|Setvelocity (* (+ (Variables|Default|Getvelocity) (* vel (Variables|Default|Getboost))) (/ _maxvelocity (Math|Vector2D|Vector2DLength (+ (Variables|Default|Getvelocity) (* vel (Variables|Default|Getboost)))))))
    (else
      (Variables|Default|Setvelocity (+ (Variables|Default|Getvelocity) (* vel (Variables|Default|Getboost)))))))

(fn Slowdown
  (if (> (Math|Vector2D|Vector2DLength (Variables|Default|Getvelocity)) (Variables|Default|Getslowing))
    (Variables|Default|Setvelocity (- (Variables|Default|Getvelocity) (* (Math|Vector2D|Normalize2D (Variables|Default|Getvelocity)) (Variables|Default|Getslowing))))
    (else
      (Variables|Default|Setvelocity ""))))

(fn Shot
  (params (indexWeapon :type Integer) (Aim :type Vector))
  (Default|Shot (Utilities|Array|Get(acopy) (Variables|Default|Getweapons) indexWeapon) Aim))

(fn SpawnWeapons
  (for _array_element (Variables|Default|GetweaponClasses)
    (if (Utilities|IsValidClass _array_element)
      (bind _returnvalue (Game|SpawnActorfromClass _array_element (Math|Transform|MakeTransform (Transformation|GetActorLocation)) "AlwaysSpawn" 0 0))
      (Transformation|AttachActorToActor _returnvalue self "None" "KeepWorld" "KeepRelative" "KeepRelative" true)
      (Utilities|Array|Add (Variables|Default|Getweapons) _returnvalue)
      (Default|InitWeapon _returnvalue (Variables|Default|GetGod) self)
      (else
        (Utilities|Array|Add (Variables|Default|Getweapons) 0)))))

(fn Init
  (params (God :type BP%20Player%20Pawn%20Object%20Reference))
  (|CallParentFunction God)
  (CallFunction|SpawnWeapons))

(fn Death
  (Default|PlayerDeath (Variables|Default|GetGod) self)
  (for _array_element (Variables|Default|Getweapons)
    (Utilities|IsValid _array_element
      (:Is%20Valid
        (CallFunction|Death _array_element))))
  (|CallParentFunction))

(fn Touch
  (params (other :type BP%20Game%20Actor%20Object%20Reference) (impulse :type Vector :default "0, 0, 0"))
  (|CallParentFunction other impulse)
  (Variables|Default|Setvelocity (+ (Variables|Default|Getvelocity) (Math|Conversions|ToVector2D(Vector) (* impulse 1.0)))))

(fn TicktoThink
  (params (deltaTime :type Float%20%28single-precision%29))
  (bind _output_get (Variables|Default|SetTtf (- (Variables|Default|GetTtf) deltaTime)))
  (if (and (< _output_get 0.0) (not (Variables|Default|GetisPlayer)))
    (Variables|Default|Setttf (Variables|Default|GetTicksToThink))
    (CallFunction|Think)))

(fn Think
  (bind _mainplayer (Variables|Default|GetmainPlayer))
  (bind _returnvalue (Transformation|GetActorLocation _mainplayer))
  (Utilities|IsValid (Variables|Default|GetmainPlayer)
    (:Is%20Valid
      _)
    (:Is%20Not%20Valid
      (CallFunction|ResetMain)
      (Utilities|IsValid _mainplayer
        (:Is%20Valid
          _)
        (:Is%20Not%20Valid
          (return)))))
  (Variables|Default|SetAimToMove (+ _returnvalue (* (Math|Vector|RotateVectorAroundAxis (Math|Vector|Normalize (- (Transformation|GetActorLocation) _returnvalue)) (Math|Random|RandomFloatinRange -2e+01 2e+01) "0, 0,1.000000") (Variables|Default|GetBestLenToFriend)))))

(fn TryShoting
  (bind _returnvalue (Transformation|GetActorLocation))
  (for (_array_element _array_index) (Variables|Default|Getweapons)
    (if (Utilities|IsValid _array_element)
      (bind _canshot (Default|IsCanShot _array_element))
      (if _canshot
        (bind _target (CallFunction|GetIdealEnemy _returnvalue (Variables|/Game/Blueprints/Weapons/BP_WeaponBase.BP_WeaponBase_C|GetdistanceMin _array_element) (Variables|/Game/Blueprints/Weapons/BP_WeaponBase.BP_WeaponBase_C|GetdistanceMax _array_element) (Variables|/Game/Blueprints/Weapons/BP_WeaponBase.BP_WeaponBase_C|GetdistanceIdeal _array_element)))
        (Utilities|IsValid _target
          (:Is%20Valid
            (CallFunction|Shot _array_index (- (Transformation|GetActorLocation _target) _returnvalue))))))))

(fn GetIdealEnemy
  (params (Pos :type Vector) (minDis :type Float%20%28single-precision%29) (maxDis :type Float%20%28single-precision%29) (idealDis :type Float%20%28single-precision%29))
  (bind _enemies (Default|GetEnemies (Variables|Default|GetGod)))
  (for (_array_element _array_index) _enemies
    (if (|(((min<0)||(max<0))||((len>=min)&&(len<=max))) (Utilities|Lengthto Pos _array_element) minDis maxDis)
      (if (== (LocalVariables|GetMinIndex) -1)
        (LocalVariables|SetMinLength (|(abs((a-b))) (Utilities|Lengthto Pos _array_element) idealDis) :!label _label)
        (LocalVariables|SetMinIndex _array_index)
        (elif (< (|(abs((a-b))) (Utilities|Lengthto Pos _array_element) idealDis) (LocalVariables|GetMinLength))
          (goto _label)))))
  (if (== (LocalVariables|GetMinIndex) -1)
    (return 0)
    (else
      (return (Utilities|Array|Get(acopy) _enemies (LocalVariables|GetMinIndex))))))

(fn SetIsPlayer
  (params (isPlayer :type Boolean))
  (bind _output_get (Variables|Default|SetisPlayer isPlayer))
  (if (and (== (Variables|Default|GetmainPlayer) self) (not _output_get))
    (CallFunction|ResetMain)))

(fn ResetMain
  (Variables|Default|SetmainPlayer (Variables|/Game/Blueprints/BP_PlayerPawn.BP_PlayerPawn_C|GetActivePlayer (Variables|Default|GetGod))))